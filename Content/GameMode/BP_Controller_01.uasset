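; BP_Controller_01 is a controller Blueprint that handles the screen fade-in and HUD setup when play begins.
; On BeginPlay it holds the camera at full black for a short delay, then runs a timed camera fade to clear and releases the manual fade once that finishes.
; Partway through the fade, a parallel sequence branch creates the BPW_HUD_Main widget and adds it to the viewport.
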(event EventBeginPlay
  (bind _returnvalue (Game|GetPlayerCameraManager 0))
  (Utilities|FlowControl|Sequence
    (:then_0
      (Class|PlayerCameraManager|SetManualCameraFade :self _returnvalue :InFadeAmount 1.0)
      (Utilities|FlowControl|Delay 2.0)
      (CameraFades|StartCameraFade :self _returnvalue :FromAlpha 1.0 :ToAlpha 0.0 :Duration 3.0)
      (Utilities|FlowControl|Sequence
        (:then_0
          (Utilities|FlowControl|Delay 3.0)
          (Class|PlayerCameraManager|SetManualCameraFade :self _returnvalue :InFadeAmount 0.0))
        (:then_1
          (Utilities|FlowControl|Delay 1.5)
          (bind _returnvalue_2 (UserInterface|CreateWidget "/Game/Widget/BPW_HUD_Main.BPW_HUD_Main_C"))
          (UserInterface|Viewport|AddtoViewport _returnvalue_2 0))))))

(fn ConstructionScript)