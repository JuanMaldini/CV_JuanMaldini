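; Pawn that steps a rotator gizmo in 60-degree yaw turns, apparently to browse six résumé sections like Skills and Education.
; Left/Right inputs or the RotateGizmo event call UpdateRotation to set start and target rotations.
; A Timeline lerps between them, with a Continue flag blocking new turns until it finishes.
; The construction script applies one shared arm length to the six section arms.
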(event Custom|Rotate%20Gizmo
  (params (Positive :type Boolean))
  (if (Variables|Default|Get%20Continue)
    (Variables|Default|Set%20Continue false)
    (CallFunction|UpdateRotation Positive)
    (bind _0_1 (Timeline|Timeline PlayFromStart)
      (:Update
        (Transformation|SetRelativeRotation (Variables|Default|GetGizmo-Rotator) (Math|Rotator|Lerp(Rotator) (Variables|Default|GetRotation%20Actual) (Variables|Default|GetRotation%20Target) _0_1) false false))
      (:Finished
        (Variables|Default|Set%20Continue true)))))

(event Input|ActionEvents|InputActionLeftAction
  (params (Key :type Key%20Structure :default "None"))
  (:Pressed
    (if (Variables|Default|Get%20Continue)
      (Variables|Default|Set%20Continue false)
      (CallFunction|UpdateRotation true)
      (bind _0_1 (Timeline|Timeline PlayFromStart)
        (:Update
          (Transformation|SetRelativeRotation (Variables|Default|GetGizmo-Rotator) (Math|Rotator|Lerp(Rotator) (Variables|Default|GetRotation%20Actual) (Variables|Default|GetRotation%20Target) _0_1) false false))
        (:Finished
          (Variables|Default|Set%20Continue true))))))

(event Input|ActionEvents|InputActionRightAction
  (params (Key :type Key%20Structure :default "None"))
  (:Pressed
    (if (Variables|Default|Get%20Continue)
      (Variables|Default|Set%20Continue false)
      (CallFunction|UpdateRotation false)
      (bind _0_1 (Timeline|Timeline PlayFromStart)
        (:Update
          (Transformation|SetRelativeRotation (Variables|Default|GetGizmo-Rotator) (Math|Rotator|Lerp(Rotator) (Variables|Default|GetRotation%20Actual) (Variables|Default|GetRotation%20Target) _0_1) false false))
        (:Finished
          (Variables|Default|Set%20Continue true))))))

(fn ConstructionScript
  (bind _arm_lenght (Variables|Default|GetArm%20Lenght))
  (Variables|/Script/Engine.SpringArmComponent|SetTargetArmLength (Variables|Default|Get01-Personal%20information%20) _arm_lenght)
  (Variables|/Script/Engine.SpringArmComponent|SetTargetArmLength (Variables|Default|Get04-Skills) _arm_lenght)
  (Variables|/Script/Engine.SpringArmComponent|SetTargetArmLength (Variables|Default|Get03-Experience) _arm_lenght)
  (Variables|/Script/Engine.SpringArmComponent|SetTargetArmLength (Variables|Default|Get06-Find%20me) _arm_lenght)
  (Variables|/Script/Engine.SpringArmComponent|SetTargetArmLength (Variables|Default|Get02-Education) _arm_lenght)
  (Variables|/Script/Engine.SpringArmComponent|SetTargetArmLength (Variables|Default|Get05-Icons) _arm_lenght))

(fn UpdateRotation
  (params (Direction :type Boolean))
  (Variables|Default|SetRotation%20Actual (.rotation (Transformation|GetRelativeTransform (Variables|Default|GetGizmo-Rotator))))
  (if Direction
    (Variables|Default|SetRotation%20Target (Math|Rotator|MakeRotator (.roll (Variables|Default|GetRotation%20Actual)) (.pitch (Variables|Default|GetRotation%20Actual)) (+ (.yaw (Variables|Default|GetRotation%20Actual)) 6e+01)))
    (else
      (Variables|Default|SetRotation%20Target (Math|Rotator|MakeRotator (.roll (Variables|Default|GetRotation%20Actual)) (.pitch (Variables|Default|GetRotation%20Actual)) (- (.yaw (Variables|Default|GetRotation%20Actual)) 6e+01)))))
  (return))