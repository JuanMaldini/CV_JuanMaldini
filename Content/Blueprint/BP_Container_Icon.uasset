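; BP_Container_Icon is a Blueprint that spawns physical icon actors at the player pawn's Container.
; Its Spawn_Icons event casts the player pawn to BP_Pawn_01 and creates a scaled-down BP_Icon at the Container's world location, randomly offset in Y and Z up to RangeRandom.
; Each new icon's static mesh receives a small upward impulse.
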(event Custom|Spawn_Icons
  (bind _range_random (Variables|Default|GetRange%20Random))
  (bind _returnvalue (Math|Random|RandomFloatinRange 0.0 _range_random))
  (bind _asbp_pawn_01 (Utilities|Casting|CastToBP_Pawn_01 (Game|Player|GetPlayerPawn 0)))
  (bind _returnvalue_2 (Game|SpawnActorfromClass "/Game/Blueprint/BP_Icon.BP_Icon_C" (Math|Transform|MakeTransform (+ (Transformation|GetWorldLocation (Variables|/Game/GameMode/BP_Pawn_01.BP_Pawn_01_C|GetContainer _asbp_pawn_01)) (Math|Vector|MakeVector 0.0 _returnvalue _returnvalue)) "0, 0, 0" "0.400000,0.400000,0.400000") "Undefined" 0 0))
  (Physics|AddImpulse (Variables|/Game/Blueprint/BP_Icon.BP_Icon_C|GetStaticMesh _returnvalue_2) "0.000000,0.000000,100.000000" "None" false))

(fn ConstructionScript)